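; Spline-based Wwise sound test actor that moves one or two emitters along a path relative to the player character.
; Single mode eases the emitter toward a target location; dual mode snaps the first to the closest spline point and conditionally moves the second to a mirrored point index.
; Collision spheres sized to the attenuation radius post play/stop events on player overlap.
; Optional sphere meshes and debug drawing visualise the setup.
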(event OnComponentBeginOverlap(Event_Collision)
  (params (OverlappedComponent :type Primitive%20Component%20Object%20Reference) (OtherActor :type Actor%20Object%20Reference) (OtherComp :type Primitive%20Component%20Object%20Reference) (OtherBodyIndex :type Integer) (bFromSweep :type Boolean) (SweepResult :type Hit%20Result%20Structure%20%28by%20ref%29))
  ;[1 1 1] Emitter One Sounds
  (if (== OtherActor (Variables|Components|GetCharacter))
    (if (Variables|Default|GetPlaySoundEmitterOne)
      (Class|AkGameObject|PostAkEvent (Variables|Default|GetPlay_Event) "/Game/Wwise/Event/DefaultWorkUnit/Play_Event.Play_Event"))))

(event OnComponentEndOverlap(Event_Collision)
  (params (OverlappedComponent :type Primitive%20Component%20Object%20Reference) (OtherActor :type Actor%20Object%20Reference) (OtherComp :type Primitive%20Component%20Object%20Reference) (OtherBodyIndex :type Integer))
  ;[1 1 1] Emitter One Sounds
  (if (== OtherActor (Variables|Components|GetCharacter))
    (if (Variables|Default|GetPlaySoundEmitterOne)
      (Class|AkGameObject|PostAkEvent (Variables|Default|GetPlay_Event) "/Game/Wwise/Event/DefaultWorkUnit/Stop_Event.Stop_Event"))))

(event OnComponentBeginOverlap(Event1_Collision)
  (params (OverlappedComponent :type Primitive%20Component%20Object%20Reference) (OtherActor :type Actor%20Object%20Reference) (OtherComp :type Primitive%20Component%20Object%20Reference) (OtherBodyIndex :type Integer) (bFromSweep :type Boolean) (SweepResult :type Hit%20Result%20Structure%20%28by%20ref%29))
  ;[1 1 1] Emitter Two Sounds
  (if (== OtherActor (Variables|Components|GetCharacter))
    (if (Variables|Default|GetPlaySoundEmitterTwo)
      (Class|AkGameObject|PostAkEvent (Variables|Default|GetPlay_Event1) "/Game/Wwise/Event/DefaultWorkUnit/Play_Event.Play_Event"))))

(event OnComponentEndOverlap(Event1_Collision)
  (params (OverlappedComponent :type Primitive%20Component%20Object%20Reference) (OtherActor :type Actor%20Object%20Reference) (OtherComp :type Primitive%20Component%20Object%20Reference) (OtherBodyIndex :type Integer))
  ;[1 1 1] Emitter Two Sounds
  (if (== OtherActor (Variables|Components|GetCharacter))
    (if (Variables|Default|GetPlaySoundEmitterTwo)
      (Class|AkGameObject|PostAkEvent (Variables|Default|GetPlay_Event1) "/Game/Wwise/Event/DefaultWorkUnit/Stop_Event.Stop_Event"))))

(event EventBeginPlay
  (bind _spline (Variables|Default|GetSpline))
  (bind _play_event1 (Variables|Default|GetPlay_Event1))
  ;[1 1 1] BeginPlay
  (Utilities|FlowControl|Sequence
    (:then_0
      (bind _asthird_person_character (Utilities|Casting|CastToThirdPersonCharacter (Game|GetPlayerCharacter 0)))
      (Variables|Components|SetCharacter _asthird_person_character)
      (Variables|Default|SetWwiseAttenuationRadius (Class|AkComponent|GetAttenuationRadius (Variables|Default|GetPlay_Event))))
    (:then_1
      (if (Variables|Default|GetTwoEmitters)
        (Transformation|SetWorldLocation _play_event1 (Class|SplineComponent|GetLocationatSplineInputKey _spline (Math|Conversions|ToFloat(Integer) (Spline|GetNumberOfSplinePoints _spline)) "World") false false)
        (bind _returnvalue (Utilities|DistancetoChar _play_event1))
        (Variables|Default|SetEmitterTwoDistanceToChar _returnvalue)))))

(event EventTick
  (params (DeltaSeconds :type Float%20%28single-precision%29))
  (bind _play_event (Variables|Default|GetPlay_Event))
  (bind _returnvalue (Transformation|GetWorldLocation _play_event))
  (Utilities|StartEndDrawDebug)
  (if (Variables|Default|GetTwoEmitters)
    ;[1 1 1] Two Emitters
    (Utilities|EmitterOne)
    (if (not (> (Variables|Default|GetEmitterOneDistanceToChar) (Variables|Default|GetWwiseAttenuationRadius)))
      (if (> (Variables|Default|GetEmitterOneDistanceToChar) (Variables|Default|GetThreshold%20distance))
        (Utilities|EmitterTwo)))
    (else
      ;[1 1 1] One Emiter
      (Components|Sphere|SetSphereRadius (Variables|Default|GetEvent_Collision) (Variables|Default|GetWwiseAttenuationRadius) true)
      (Transformation|SetWorldLocation _play_event (Math|Interpolation|VInterpTo _returnvalue (Utilities|FindLocationtoWorldLocation) (Utilities|Time|GetWorldDeltaSeconds) (Variables|Default|GetInterpolationSpeed)) false false)
      (Utilities|DrawDebuger _returnvalue "(R=1.000000,G=0.000000,B=0.081195,A=1.000000)"))))

(fn ConstructionScript
  (Utilities|StartEndDrawDebug)
  (CallFunction|SpawnPoints))

(fn SpawnPoints
  (if (Variables|DebugDraw|GetSpawnMeshes)
    (for _index (range 0 (Variables|DebugDraw|GetNumbsMesh))
      (bind _returnvalue (AddComponent|AddStaticMeshComponent false (Math|Transform|MakeTransform (Spline|GetLocationatTime (Variables|Default|GetSpline) (* (Math|Conversions|ToFloat(Integer) _index) 0.1) "Local" false) "0, 0, 0" "1,1,1")))
      (Transformation|SetRelativeScale3D _returnvalue "0.500000,0.500000,0.500000")
      (Rendering|Material|SetMaterial _returnvalue 0 "/Engine/MapTemplates/Materials/BasicAsset01.BasicAsset01")
      (Components|StaticMesh|SetStaticMesh _returnvalue "/Engine/EngineMeshes/Sphere.Sphere"))
    (else
      (return))))