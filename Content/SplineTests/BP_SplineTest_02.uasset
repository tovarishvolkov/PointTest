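; BP_SplineTest_02 is a test actor that places sphere static mesh components along its spline.
; SpawnObjects samples the spline at 0.1 time steps in local space without constant velocity, adding a sphere at each point.
; Tick calls it every frame, so components keep accumulating, while the construction script's call is disconnected.
; ControlPoints defines a straight two-point spline along X but is not called in this file.
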(event EventBeginPlay)

(event Collision|EventActorBeginOverlap
  (params (OtherActor :type Actor%20Object%20Reference)))

(event EventTick
  (params (DeltaSeconds :type Float%20%28single-precision%29))
  (CallFunction|SpawnObjects (Variables|Default|GetSpline)))

(fn ConstructionScript)

(fn ControlPoints
  (params (Spline :type Spline%20Component%20Object%20Reference))
  (Spline|SetSplinePoints Spline (Utilities|Array|MakeArray "0, 0, 0" "1000.000000, 0, 0") "Local" true))

(fn SpawnObjects
  (params (NewParam :type Spline%20Component%20Object%20Reference))
  (for _index (range 0 10)
    (bind _returnvalue (AddComponent|AddStaticMeshComponent false (Math|Transform|MakeTransform (Spline|GetLocationatTime NewParam (* _index 0.1) "Local" false) "0, 0, 0" "1,1,1")))
    (Components|StaticMesh|SetStaticMesh _returnvalue "/Engine/EngineMeshes/Sphere.Sphere")))