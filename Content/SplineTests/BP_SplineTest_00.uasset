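; BP_SplineTest_00 is a test actor that moves a sphere along a spline.
; Every Tick it sets a slowed timeline play rate and calls Play, and each update places the sphere at the spline point for the timeline's time.
; Each update also debug-draws a visibility line trace from the sphere to the player pawn, without using the hit result.
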(event EventBeginPlay)

(event Collision|EventActorBeginOverlap
  (params (OtherActor :type Actor%20Object%20Reference)))

(event EventTick
  (params (DeltaSeconds :type Float%20%28single-precision%29))
  (bind _sphere (Variables|Default|GetSphere))
  (Components|Timeline|SetPlayRate (Variables|Default|GetTimeline_0) 0.1)
  (bind _time (Timeline|Timeline_0 Play)
    (:Update
      (Transformation|SetRelativeLocation _sphere (Spline|GetLocationatTime (Variables|Default|GetSpline) _time "Local" false) false false)
      (Collision|LineTraceByChannel (Transformation|GetWorldLocation _sphere) (Transformation|GetActorLocation (Game|Player|GetPlayerPawn 0)) "TraceTypeQuery1" false 0 "ForOneFrame"))))

(fn ConstructionScript)