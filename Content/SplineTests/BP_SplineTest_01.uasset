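; Spline test actor that rebuilds a spline and debug-traces toward the player controller every Tick.
; ControlPoints resets the spline to run from local origin to Spherelocation with a linear end point.
; SpawnPoints spawns nothing: per index it shifts the spline component by a sampled location, at distances not scaled by spline length.
; It also sets Sphere to a cube mesh and draws an unused visibility trace from it.
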(event Collision|EventActorBeginOverlap
  (params (OtherActor :type Actor%20Object%20Reference)))

(event EventTick
  (params (DeltaSeconds :type Float%20%28single-precision%29))
  (bind _spline (Variables|Default|GetSpline))
  (bind _outputpin (CallFunction|ControlPoints _spline))
  (CallFunction|SpawnPoints (Spline|GetNumberOfSplinePoints _spline) _outputpin))

(fn ConstructionScript)

(fn ControlPoints
  (params (InputPin :type Spline%20Component%20Object%20Reference))
  (Spline|SetSplinePoints InputPin (Utilities|Array|MakeArray "0, 0, 0" (Variables|Default|GetSpherelocation)) "Local" true)
  (Spline|SetSplinePointType InputPin 1 "Linear" true)
  (return InputPin))

(fn SpawnPoints
  (params (InInt :type Integer) (Target :type Spline%20Component%20Object%20Reference))
  (bind _sphere (Variables|Default|GetSphere))
  (for _index (range 0 InInt)
    (Transformation|AddLocalOffset Target (Spline|GetLocationatDistanceAlongSpline Target (* (Math|Conversions|ToFloat(Integer) _index) (/ 1.0 (Math|Conversions|ToFloat(Integer) InInt))) "Local") false false)
    (Components|StaticMesh|SetStaticMesh _sphere "/Engine/VREditor/BasicMeshes/SM_Cube_01.SM_Cube_01")
    (Collision|LineTraceByChannel (Transformation|GetWorldLocation _sphere) (Transformation|GetActorLocation (Game|GetPlayerController 0)) "TraceTypeQuery1" false 0 "ForOneFrame")))