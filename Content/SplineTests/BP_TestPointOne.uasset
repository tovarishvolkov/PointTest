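; Test actor for a spline whose end point tracks the player, with heavy debug drawing.
; Each Tick rebuilds a two-point spline, then moves point 1 to the player's X plus an offset, clamped between two bounds, with Y and Z sampled along the spline.
; A debug trace links that point to the player.
; Runtime spline creation and SpawnPionts are unwired, and both overlap events set and print Chr as true.
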(event EventBeginPlay)

(event Collision|EventActorBeginOverlap
  (params (OtherActor :type Actor%20Object%20Reference))
  (bind _output_get (Variables|Default|SetChr true))
  (Development|PrintString (Utilities|String|ToString(Boolean) _output_get)))

(event EventTick
  (params (DeltaSeconds :type Float%20%28single-precision%29))
  (bind _returnvalue (Game|GetPlayerCharacter 0))
  (bind _spline (Variables|Default|GetSpline))
  (bind _spline_2 (Variables|Default|GetSpline))
  (bind _returnvalue_2 (Transformation|GetActorLocation _returnvalue))
  (bind _returnvalue_3 (+ _returnvalue_2 "200.000000, 0, 0"))
  (bind _returnvalue_4 (Spline|GetLocationatDistanceAlongSpline _spline (.x _returnvalue_3) "World"))
  (Development|PrintString (Utilities|String|ToString(Integer) (Spline|GetNumberOfSplinePoints (Variables|Default|GetSpline))))
  (Rendering|Debug|DrawDebugString _returnvalue_2 (Utilities|String|ToString(Float) (.x _returnvalue_3)) 0 "(R=0.097119,G=1.000000,B=0.000000,A=1.000000)")
  (Variables|Default|SetVector_0 (Math|Vector|MakeVector (Math|Float|Clamp(Float) (.x _returnvalue_3) (.x (Variables|Default|GetVector_2)) (.x (Variables|Default|GetVector_1))) (.y _returnvalue_4) (.z _returnvalue_4)))
  (bind _outputpin (CallFunction|ControlPoints _spline_2))
  (Rendering|Debug|DrawDebugSphere (Spline|GetLocationatSplinePoint _outputpin 1 "World") 1e+02 12 "(R=1.000000,G=0.224327,B=0.265147,A=1.000000)" 0.0)
  (Collision|LineTraceByChannel (Spline|GetLocationatSplinePoint _outputpin 1 "World") (Transformation|GetActorLocation (Game|GetPlayerCharacter 0)) "TraceTypeQuery1" false 0 "ForOneFrame")
  (Spline|SetLocationatSplinePoint _spline_2 1 (Math|Vector|MakeVector (.x (+ (Variables|Default|GetVector_0) "0, 0, 0")) (.y (+ (Variables|Default|GetVector_0) "0, 0, 0")) (.z (+ (Variables|Default|GetVector_0) "0, 0, 0"))) "World" true)
  (Rendering|Debug|DrawDebugString (Spline|GetLocationatSplinePoint _outputpin 1 "World") (Utilities|String|ToString(Vector) (Spline|GetLocationatSplinePoint _outputpin 1 "World")) 0 "(R=1.000000,G=1.000000,B=1.000000,A=1.000000)"))

(event Collision|EventActorEndOverlap
  (params (OtherActor :type Actor%20Object%20Reference))
  (bind _output_get (Variables|Default|SetChr true))
  (Development|PrintString (Utilities|String|ToString(Boolean) _output_get)))

(fn ConstructionScript)

(fn CreateSplines
  (bind _returnvalue (AddComponent|AddSplineComponent false))
  (return _returnvalue))

(fn ControlPoints
  (params (Spline :type Spline%20Component%20Object%20Reference))
  (bind _returnvalue (Spline|GetLocationatSplinePoint Spline 2 "World"))
  (bind _returnvalue_2 (Spline|GetLocationatSplinePoint Spline 0 "World"))
  (bind _output_get (Variables|Default|SetSplinePoints (Utilities|Array|MakeArray "0, 0, 0" (Variables|Default|GetVector_0))))
  (Spline|SetSplinePoints Spline _output_get "Local" true)
  (Rendering|Debug|DrawDebugString _returnvalue_2 (Utilities|String|ToString(Vector) _returnvalue_2) 0 "(R=1.000000,G=0.000000,B=0.892491,A=1.000000)")
  (Rendering|Debug|DrawDebugString _returnvalue (Utilities|String|ToString(Vector) _returnvalue) 0 "(R=0.533860,G=1.000000,B=0.000000,A=1.000000)")
  (Spline|SetSplinePointType Spline 1 "Linear" true)
  (return Spline))

(fn SpawnPionts
  (params (Spline :type Spline%20Component%20Object%20Reference) (PointsCount :type Integer))
  (for _index (range 0 PointsCount)
    (Transformation|AddLocalOffset Spline (Spline|GetLocationatTime Spline (* (Math|Conversions|ToFloat(Integer) _index) (/ 1.0 (Math|Conversions|ToFloat(Integer) PointsCount))) "Local" true) false false)))