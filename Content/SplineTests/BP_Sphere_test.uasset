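; BP_Sphere_test is a spline test actor that follows the player pawn along the world X axis.
; Each Tick it copies the pawn's X into its own location while keeping its Y and Z.
; It then calls DrawDebug, which draws a line from the actor to the pawn, a sphere at the actor and its coordinates as text above it.
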(event EventBeginPlay)

(event Collision|EventActorBeginOverlap
  (params (OtherActor :type Actor%20Object%20Reference)))

(event EventTick
  (params (DeltaSeconds :type Float%20%28single-precision%29))
  (bind _returnvalue (Game|Player|GetPlayerPawn 0))
  (bind _self self)
  (bind _returnvalue_2 (Transformation|GetActorLocation _self))
  (Transformation|SetActorLocation _self (Math|Vector|MakeVector (.x (Transformation|GetActorLocation _returnvalue)) (.y _returnvalue_2) (.z _returnvalue_2)) false false)
  (Utilities|DrawDebug (Transformation|GetActorLocation _self) (Transformation|GetActorLocation _returnvalue)))

(fn ConstructionScript)